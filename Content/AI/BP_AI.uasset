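; AI pawn Blueprint that spots the player and performs a shove attack.
; PawnSensing sets the seeingPlayer Blackboard key to true when it sees a pawn tagged Player; nothing here clears it.
; The AttackPlayer event plays a push/shove montage on the mesh, guarded by an Attacking flag that resets only when the montage completes.
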(event OnSeePawn(PawnSensing)
  (params (Pawn :type Pawn%20Object%20Reference))
  (if (Actor|ActorHasTag Pawn "Player")
    (AI|Components|Blackboard|SetValueasBool (AI|GetBlackboard (AI|GetAIController self)) (Utilities|Name|MakeLiteralName "seeingPlayer") true)))

(event Custom|AttackPlayer
  (if (not (Variables|Default|GetAttacking))
    (Variables|Default|SetAttacking true)
    (Animation|Montage|PlayMontage (Variables|Character|GetMesh) "/Game/AI/Paired_PushShove_Att_Montage.Paired_PushShove_Att_Montage"
      (:OnCompleted
        (Variables|Default|SetAttacking false)))))

(fn ConstructionScript)